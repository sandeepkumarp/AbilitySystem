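; BP_PlayerControllerBase is a base player controller that turns movement and jump input into actions on the controlled pawn.
; MoveForward and MoveRight axes add movement input along the camera manager's forward and right vectors, making movement camera-relative.
; Pressing Jump casts the pawn to BP_CharacterBase and calls Jump, doing nothing for other pawn types.
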(event `InputAxis|MoveForward`
  (params (AxisValue :type "Float (single-precision)"))
  (`Pawn.AddMovementInput` (`self.K2_GetPawn`) (`KismetMathLibrary.GetForwardVector` (`PlayerCameraManager.GetCameraRotation` (`self.PlayerCameraManager`))) AxisValue false))

(event `InputAxis|MoveRight`
  (params (AxisValue :type "Float (single-precision)"))
  (`Pawn.AddMovementInput` (`self.K2_GetPawn`) (`KismetMathLibrary.GetRightVector` (`PlayerCameraManager.GetCameraRotation` (`self.PlayerCameraManager`))) AxisValue false))

(event `InputAction|Jump`
  (params (Key :type "Key Structure"))
  (:`Pressed`
    (bind _asbp_character_base (cast `/Game/Blueprints/Characters/BP_CharacterBase` (`self.K2_GetPawn`)))
    (`Character.Jump` _asbp_character_base)))

(fn `UserConstructionScript`)